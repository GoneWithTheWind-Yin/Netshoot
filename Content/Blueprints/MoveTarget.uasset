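; MoveTarget is a moving target that awards score to the player who damages it.
; Each tick it moves its Sphere component upward from the actor's location by Speed, snapping the height back to a low starting Z once an upper limit is passed.
; On any damage, it casts the instigator's PlayerState to MyPlayerState and calls IncrementScore, regardless of damage amount.
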(event EventTick
  (params (DeltaSeconds :type Float%20%28single-precision%29))
  (bind _returnvalue (Transformation|GetActorLocation))
  (bind _sphere (Variables|Default|GetSphere))
  (if (<= (.z _returnvalue) 3e+02)
    (Transformation|SetWorldLocation _sphere (Math|Vector|MakeVector (.x _returnvalue) (.y _returnvalue) (+ (.z _returnvalue) (Variables|Default|Getspeed))) false false)
    (else
      (Transformation|SetWorldLocation _sphere (Math|Vector|MakeVector (.x _returnvalue) (.y _returnvalue) 8e+01) false false))))

(event Game|Damage|EventAnyDamage
  (params (Damage :type Float%20%28single-precision%29) (DamageType :type Damage%20Type%20Object%20Reference) (InstigatedBy :type Controller%20Object%20Reference) (DamageCauser :type Actor%20Object%20Reference))
  (bind _asmy_player_state (Utilities|Casting|CastToMyPlayerState (Variables|/Script/Engine.Controller|GetPlayerState InstigatedBy)))
  (Default|IncrementScore _asmy_player_state))

(fn ConstructionScript)